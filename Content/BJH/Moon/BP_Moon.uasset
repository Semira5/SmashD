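; BP_Moon is a moon actor that spins continuously in the level.
; Its construction script orients the whole actor so its forward X axis points toward an Origin point.
; Each Tick adds a small fixed step to the Moon component's relative yaw, without delta-time scaling, so spin speed depends on frame rate.
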(event EventBeginPlay)

(event Collision|EventActorBeginOverlap
  (params (OtherActor :type Actor%20Object%20Reference)))

(event EventTick
  (params (DeltaSeconds :type Float%20%28single-precision%29))
  (bind _moon (Variables|Default|GetMoon))
  (bind _relativerotation (Variables|/Script/Engine.SceneComponent|GetRelativeRotation _moon))
  ;[1 1 1] 달 회전
  (Transformation|SetRelativeRotation _moon (Math|Rotator|MakeRotator (.roll _relativerotation) (.pitch _relativerotation) (+ (.yaw _relativerotation) 0.1)) false false))

(fn ConstructionScript
  (Transformation|SetActorRotation (Math|Conversions|RotationFromXVector (Math|Vector|Normalize (- (Variables|Default|GetOrigin) (Transformation|GetActorLocation))))))