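; BP_OSY_Crash is a drum-set actor, apparently a crash cymbal, that plays a water effect when a SmashCharacter touches it.
; An overlap on its box component spawns the effect system at a fixed offset from the actor's location, using the actor's rotation.
; A Wait flag blocks retriggering during a short delay, after which the effect component is destroyed and the flag resets.
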(event OnComponentBeginOverlap(compBox)
  (params (OverlappedComponent :type Primitive%20Component%20Object%20Reference) (OtherActor :type Actor%20Object%20Reference) (OtherComp :type Primitive%20Component%20Object%20Reference) (OtherBodyIndex :type Integer) (bFromSweep :type Boolean) (SweepResult :type Hit%20Result%20Structure%20%28by%20ref%29))
  (Utilities|Casting|CastToSmashCharacter OtherActor)
  (if (Variables|Default|GetWait)
    (bind _returnvalue (Niagara|SpawnSystematLocation "/Game/BJH/Effect/WaterEffect.WaterEffect" (+ (Transformation|GetActorLocation) "-70.000000,-20.000000,270.000000") (Transformation|GetActorRotation)))
    (Variables|Default|SetWait false)
    (Utilities|FlowControl|Delay 0.5)
    (Components|DestroyComponent _returnvalue)
    (Variables|Default|SetWait true)))

(event EventBeginPlay)

(event Collision|EventActorBeginOverlap
  (params (OtherActor :type Actor%20Object%20Reference)))

(event EventTick
  (params (DeltaSeconds :type Float%20%28single-precision%29)))

(fn ConstructionScript)